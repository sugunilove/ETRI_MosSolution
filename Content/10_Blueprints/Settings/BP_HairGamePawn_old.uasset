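; Pawn for a hair and face viewer with orbit, pan and zoom camera, switching between Shader Rig and Hair Match views via player state dispatcher.
; Construction builds six expression head meshes with groom hair, plus mask-map and face material instances, driven by morph, animation and shader parameters.
; Hair Match shows a male or female head with one of sixteen hairstyles.
; A looping timer steps through game-instance PPG data, tinting the face's red channel.
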(event Custom|HairViewChanged
  (CallFunction|SetHairViewandSwitchFaceModel (Variables|/Script/EtriHairSolution.HairPlayerState|GetCurrentHairView (Variables|Default|GetHairPlaye%20State))))

(event EventBeginPlay
  (bind _asbp_hair_player_state (Utilities|Casting|CastToBP_HairPlayerState (Variables|Default|GetPlayerState)))
  (bind _output_get (Variables|Default|SetHairPlaye%20State _asbp_hair_player_state))
  (EventDispatchers|BindEventtoHairViewStateChangeDispatcher _output_get (delegate Custom|HairViewChanged))
  (bind _returnvalue (Utilities|Time|SetTimerbyFunctionName 0 "Apply PPG Loop Counter" (Variables|PPG|GetPPG%20Tick) true))
  (Variables|PPG|SetPPG%20TimerHandle _returnvalue))

(event Collision|EventActorBeginOverlap
  (params (OtherActor :type Actor%20Object%20Reference)))

(event EventTick
  (params (DeltaSeconds :type Float%20%28single-precision%29)))

(event EventEndPlay
  (params (EndPlayReason :type EEndPlayReason%20Enum :default "Destroyed"))
  (bind _ppg_timerhandle (Variables|PPG|GetPPG%20TimerHandle))
  (bind _hairplaye_state (Variables|Default|GetHairPlaye%20State))
  (if (Utilities|Time|IsValidTimerHandle _ppg_timerhandle)
    (Utilities|Time|ClearandInvalidateTimerbyHandle _ppg_timerhandle)
    (if (Utilities|IsValid _hairplaye_state)
      (EventDispatchers|UnbindEventfromHairViewStateChangeDispatcher _hairplaye_state (delegate Custom|HairViewChanged)))))

(event Input|ActionEvents|InputActionZoomCameraIn
  (params (Key :type Key%20Structure))
  (:Pressed
    (Variables|/Script/Engine.SpringArmComponent|SetTargetArmLength (Variables|HairPawn|CameraAction|GetCameraBoom) (Math|Float|Clamp(Float) (+ (Variables|/Script/Engine.SpringArmComponent|GetTargetArmLength (Variables|HairPawn|CameraAction|GetCameraBoom)) (Variables|HairPawn|CameraAction|GetZoom%20Tick)) (Variables|HairPawn|CameraAction|GetZoom%20Min) (Variables|HairPawn|CameraAction|GetZoom%20Max)))))

(event Input|ActionEvents|InputActionZoomCameraOut
  (params (Key :type Key%20Structure))
  (:Pressed
    (Variables|/Script/Engine.SpringArmComponent|SetTargetArmLength (Variables|HairPawn|CameraAction|GetCameraBoom) (Math|Float|Clamp(Float) (- (Variables|/Script/Engine.SpringArmComponent|GetTargetArmLength (Variables|HairPawn|CameraAction|GetCameraBoom)) (Variables|HairPawn|CameraAction|GetZoom%20Tick)) (Variables|HairPawn|CameraAction|GetZoom%20Min) (Variables|HairPawn|CameraAction|GetZoom%20Max)))))

(event Input|ActionEvents|InputActionOrbitCamera
  (params (Key :type Key%20Structure))
  ;[1 1 1] Camera Orbit (Mouse Right Click) + Pan (Mouse Center Click)
  (:Pressed
    (Variables|HairPawn|CameraAction|SetTurn%20On%20Camera%20Orbit true))
  (:Released
    (Variables|HairPawn|CameraAction|SetTurn%20On%20Camera%20Orbit false)))

(event Input|ActionEvents|InputActionPanCamera
  (params (Key :type Key%20Structure))
  ;[1 1 1] Camera Orbit (Mouse Right Click) + Pan (Mouse Center Click)
  (:Pressed
    (Variables|HairPawn|CameraAction|SetTurn%20On%20Camera%20Pan true))
  (:Released
    (Variables|HairPawn|CameraAction|SetTurn%20On%20Camera%20Pan false)))

(event Input|ActionEvents|InputActionFitsCameratoView
  (params (Key :type Key%20Structure))
  (:Pressed
    (HairPawn|CameraAction|ResetCameraTransform)))

(event Input|MouseEvents|Mouse2D
  (params (AxisValue :type Vector :default "0, 0, 0"))
  (bind (_x _y) (Math|Vector|BreakVector AxisValue))
  ;[1 1 1] Camera Orbit (Mouse Right Click) + Pan (Mouse Center Click)
  (Utilities|FlowControl|Sequence
    (:then_0
      (if (Variables|HairPawn|CameraAction|GetTurn%20On%20Camera%20Orbit)
        (Transformation|AddRelativeRotation (Variables|HairPawn|CameraAction|GetCameraBoom) (Math|Rotator|MakeRotator 0.0 0.0 _x) false false)))
    (:then_1
      (if (Variables|HairPawn|CameraAction|GetTurn%20On%20Camera%20Pan)
        (Utilities|FlowControl|Sequence
          (:then_0
            (bind _result (Math|Float|NegateFloat _x)))
          (:then_1
            (bind _result_2 (Math|Float|NegateFloat _y)))
          (:then_2
            (Transformation|AddRelativeLocation (Variables|HairPawn|CameraAction|GetFollowCamera) (Math|Vector|MakeVector 0.0 _result _result_2) false false)))))))

(fn ConstructionScript
  (Variables|/Script/Engine.SpringArmComponent|SetTargetArmLength (Variables|HairPawn|CameraAction|GetCameraBoom) (Variables|HairPawn|CameraAction|GetZoom%20Default))
  (HairPawn|Head|SkeletalMesh|InitHeadMesh)
  ;[1 1 1] PPG
  (Variables|PPG|SetPPG%20Tick (/ 1.0 6e+01))
  (bind _asbp_hair_game_instance (Utilities|Casting|CastToBP_HairGameInstance (Game|GetGameInstance)))
  (bind _output_get (Variables|PPG|SetCurrentGameInstance _asbp_hair_game_instance))
  (Variables|PPG|SetPPG%20Data (Variables|/Game/10_Blueprints/Settings/BP_HairGameInstance.BP_HairGameInstance_C|GetPPG%20Data _output_get))
  (Variables|PPG|SetPPG%20Max%20Length (Variables|/Game/10_Blueprints/Settings/BP_HairGameInstance.BP_HairGameInstance_C|GetPPG%20Max%20Length _output_get)))

(fn SetFaceMorphTarget
  (params (Weight :type Float%20%28double-precision%29))
  (Components|SkeletalMesh|SetMorphTarget (Variables|HairPawn|Head|SkeletalMesh|GetCurrentHeadMesh) (Utilities|String|StringToName (Utilities|String|EnumtoString (Variables|HairPawn|Head|GetCurrentExpression))) Weight true))

(fn ResetCameraTransform
  (bind _cameraboom (Variables|HairPawn|CameraAction|GetCameraBoom))
  (Transformation|SetRelativeLocationAndRotation _cameraboom "0, 0, 0" "0, 0, 0" false false)
  (Variables|/Script/Engine.SpringArmComponent|SetTargetArmLength _cameraboom (Variables|HairPawn|CameraAction|GetZoom%20Default))
  (Transformation|SetRelativeLocationAndRotation (Variables|HairPawn|CameraAction|GetFollowCamera) "0, 0, 0" "0, 0, 0" false false))

(fn InitHeadMesh
  (Utilities|FlowControl|Sequence
    (:then_0
      (Variables|HairPawn|Head|SetCurrentExpression "NewEnumerator6")
      ;[1 1 1] Mesh
      (bind __skeletalmeshcomponent (HairPawn|Head|SkeletalMesh|CreateandAttachHeadMesh "/Game/MetaHumans/TemplateModel/01_neutral2anger_all.01_neutral2anger_all" "/Game/MetaHumans/TemplateModel/01_neutral2anger_all_Anim.01_neutral2anger_all_Anim"))
      (bind _output_get (Variables|HairPawn|Head|SkeletalMesh|SetHeadMesh_Anger __skeletalmeshcomponent))
      (Variables|HairPawn|Head|SkeletalMesh|SetCurrentHeadMesh _output_get)
      ;[1 1 1] Mask Map
      (bind _returnvalue (Rendering|Material|CreateDynamicMaterialInstance "/Game/MetaHumans/MH_KJH/Materials/MaskMap/MI_2D_MaskMap_Anger.MI_2D_MaskMap_Anger" "None" "None" :!class /Script/Engine.KismetMaterialLibrary))
      (bind _output_get_2 (Variables|HairPawn|Head|Material|MaskMap|SetMaskMap_Anger _returnvalue))
      (Variables|HairPawn|Head|Material|MaskMap|SetCurrentMaskMapMaterial _output_get_2)
      ;[1 1 1] Shader Rig Material
      (bind _returnvalue_2 (Rendering|Material|CreateDynamicMaterialInstance "/Game/MetaHumans/MH_KJH/Materials/ShaderRig/MI_2D_Face_Anger.MI_2D_Face_Anger" "None" "None" :!class /Script/Engine.KismetMaterialLibrary))
      (bind _output_get_3 (Variables|HairPawn|Head|Material|ShaderRig|SetShaderRig_Anger _returnvalue_2))
      (Variables|HairPawn|Head|Material|ShaderRig|SetCurrentFaceShaderRigMaterial _output_get_3)
      (HairPawn|Head|Material|SwitchHeadMeshMaterial))
    (:then_1
      (bind __skeletalmeshcomponent_2 (HairPawn|Head|SkeletalMesh|CreateandAttachHeadMesh "/Game/MetaHumans/TemplateModel/02_neutral2disgust_all.02_neutral2disgust_all" "/Game/MetaHumans/TemplateModel/02_neutral2disgust_all_Anim.02_neutral2disgust_all_Anim"))
      (Variables|HairPawn|Head|SkeletalMesh|SetHeadMesh_Disgust __skeletalmeshcomponent_2)
      (bind _returnvalue_3 (Rendering|Material|CreateDynamicMaterialInstance "/Game/MetaHumans/MH_KJH/Materials/MaskMap/MI_2D_MaskMap_Disgust.MI_2D_MaskMap_Disgust" "None" "None" :!class /Script/Engine.KismetMaterialLibrary))
      (Variables|HairPawn|Head|Material|MaskMap|SetMaskMap_Disgust _returnvalue_3)
      (bind _returnvalue_4 (Rendering|Material|CreateDynamicMaterialInstance "/Game/MetaHumans/MH_KJH/Materials/ShaderRig/MI_2D_Face_Disgust.MI_2D_Face_Disgust" "None" "None" :!class /Script/Engine.KismetMaterialLibrary))
      (Variables|HairPawn|Head|Material|ShaderRig|SetShaderRig_Disgust _returnvalue_4))
    (:then_2
      (bind __skeletalmeshcomponent_3 (HairPawn|Head|SkeletalMesh|CreateandAttachHeadMesh "/Game/MetaHumans/TemplateModel/03_neutral2fear_all.03_neutral2fear_all" "/Game/MetaHumans/TemplateModel/03_neutral2fear_all_Anim.03_neutral2fear_all_Anim"))
      (Variables|HairPawn|Head|SkeletalMesh|SetHeadMesh_Fear __skeletalmeshcomponent_3)
      (bind _returnvalue_5 (Rendering|Material|CreateDynamicMaterialInstance "/Game/MetaHumans/MH_KJH/Materials/MaskMap/MI_2D_MaskMap_Fear.MI_2D_MaskMap_Fear" "None" "None" :!class /Script/Engine.KismetMaterialLibrary))
      (Variables|HairPawn|Head|Material|MaskMap|SetMaskMap_Fear _returnvalue_5)
      (bind _returnvalue_6 (Rendering|Material|CreateDynamicMaterialInstance "/Game/MetaHumans/MH_KJH/Materials/ShaderRig/MI_2D_Face_Fear.MI_2D_Face_Fear" "None" "None" :!class /Script/Engine.KismetMaterialLibrary))
      (Variables|HairPawn|Head|Material|ShaderRig|SetShaderRig_Fear _returnvalue_6))
    (:then_3
      (bind __skeletalmeshcomponent_4 (HairPawn|Head|SkeletalMesh|CreateandAttachHeadMesh "/Game/MetaHumans/TemplateModel/04_neutral2happiness_all.04_neutral2happiness_all" "/Game/MetaHumans/TemplateModel/04_neutral2happiness_all_Anim.04_neutral2happiness_all_Anim"))
      (Variables|HairPawn|Head|SkeletalMesh|SetHeadMesh_Happiness __skeletalmeshcomponent_4)
      (bind _returnvalue_7 (Rendering|Material|CreateDynamicMaterialInstance "/Game/MetaHumans/MH_KJH/Materials/MaskMap/MI_2D_MaskMap_Happniess.MI_2D_MaskMap_Happniess" "None" "None" :!class /Script/Engine.KismetMaterialLibrary))
      (Variables|HairPawn|Head|Material|MaskMap|SetMaskMap_Happy _returnvalue_7)
      (bind _returnvalue_8 (Rendering|Material|CreateDynamicMaterialInstance "/Game/MetaHumans/MH_KJH/Materials/ShaderRig/MI_2D_Face_Happiness.MI_2D_Face_Happiness" "None" "None" :!class /Script/Engine.KismetMaterialLibrary))
      (Variables|HairPawn|Head|Material|ShaderRig|SetShaderRig_Happy _returnvalue_8))
    (:then_4
      (bind __skeletalmeshcomponent_5 (HairPawn|Head|SkeletalMesh|CreateandAttachHeadMesh "/Game/MetaHumans/TemplateModel/05_neutral2sadness_all.05_neutral2sadness_all" "/Game/MetaHumans/TemplateModel/05_neutral2sadness_all_Anim.05_neutral2sadness_all_Anim"))
      (Variables|HairPawn|Head|SkeletalMesh|SetHeadMesh_Sadness __skeletalmeshcomponent_5)
      (bind _returnvalue_9 (Rendering|Material|CreateDynamicMaterialInstance "/Game/MetaHumans/MH_KJH/Materials/MaskMap/MI_2D_MaskMap_Sadness.MI_2D_MaskMap_Sadness" "None" "None" :!class /Script/Engine.KismetMaterialLibrary))
      (Variables|HairPawn|Head|Material|MaskMap|SetMaskMap_Sad _returnvalue_9)
      (bind _returnvalue_10 (Rendering|Material|CreateDynamicMaterialInstance "/Game/MetaHumans/MH_KJH/Materials/ShaderRig/MI_2D_Face_Sadness.MI_2D_Face_Sadness" "None" "None" :!class /Script/Engine.KismetMaterialLibrary))
      (Variables|HairPawn|Head|Material|ShaderRig|SetShaderRig_Sad _returnvalue_10))
    (:then_5
      (bind __skeletalmeshcomponent_6 (HairPawn|Head|SkeletalMesh|CreateandAttachHeadMesh "/Game/MetaHumans/TemplateModel/06_neutral2surprise_all.06_neutral2surprise_all" "/Game/MetaHumans/TemplateModel/06_neutral2surprise_all_Anim.06_neutral2surprise_all_Anim"))
      (Variables|HairPawn|Head|SkeletalMesh|SetHeadMesh_Surprise __skeletalmeshcomponent_6)
      (bind _returnvalue_11 (Rendering|Material|CreateDynamicMaterialInstance "/Game/MetaHumans/MH_KJH/Materials/MaskMap/MI_2D_MaskMap_Surprise.MI_2D_MaskMap_Surprise" "None" "None" :!class /Script/Engine.KismetMaterialLibrary))
      (Variables|HairPawn|Head|Material|MaskMap|SetMaskMap_Surprise _returnvalue_11)
      (bind _returnvalue_12 (Rendering|Material|CreateDynamicMaterialInstance "/Game/MetaHumans/MH_KJH/Materials/ShaderRig/MI_2D_Face_Surprise.MI_2D_Face_Surprise" "None" "None" :!class /Script/Engine.KismetMaterialLibrary))
      (Variables|HairPawn|Head|Material|ShaderRig|SetShaderRig_Surprise _returnvalue_12))
    (:then_6
      (bind _returnvalue_13 (Rendering|Material|CreateDynamicMaterialInstance "/Game/MetaHumans/MH_KJH/Materials/MaskMap/MI_2D_MaskMap_VitalSign.MI_2D_MaskMap_VitalSign" "None" "None" :!class /Script/Engine.KismetMaterialLibrary))
      (Variables|HairPawn|Head|Material|MaskMap|SetMaskMap_VitalSign _returnvalue_13)
      (bind _returnvalue_14 (Rendering|Material|CreateDynamicMaterialInstance "/Game/MetaHumans/MH_KJH/Materials/ShaderRig/MI_2D_Face_VitalSign.MI_2D_Face_VitalSign" "None" "None" :!class /Script/Engine.KismetMaterialLibrary))
      (Variables|HairPawn|Head|Material|ShaderRig|SetShaderRig_VitalSign _returnvalue_14))
    (:then_7
      (CallFunction|SetHeadMatchModelVisibility false false))))

(fn SwitchHeadMesh
  (params (Expression :type E_FaceExpression%20Enum :default "NewEnumerator6"))
  (HairPawn|Head|SkeletalMesh|ResetStateCurrentHeadMesh)
  (bind _output_get (Variables|HairPawn|Head|SetCurrentExpression Expression))
  (switch Utilities|FlowControl|Switch|SwitchonE_FaceExpression _output_get
    (:NewEnumerator6
      _)
    (:NewEnumerator0
      ;[0.07268 0.4103 1] 선택된 메시로 변경
      (Variables|HairPawn|Head|SkeletalMesh|SetCurrentHeadMesh (Variables|HairPawn|Head|SkeletalMesh|GetHeadMesh_Anger))
      (HairPawn|Head|Material|SwitchHeadMeshMaterial :!label _label))
    (:NewEnumerator1
      (Variables|HairPawn|Head|SkeletalMesh|SetCurrentHeadMesh (Variables|HairPawn|Head|SkeletalMesh|GetHeadMesh_Disgust))
      (goto _label))
    (:NewEnumerator2
      (Variables|HairPawn|Head|SkeletalMesh|SetCurrentHeadMesh (Variables|HairPawn|Head|SkeletalMesh|GetHeadMesh_Fear))
      (goto _label))
    (:NewEnumerator3
      (Variables|HairPawn|Head|SkeletalMesh|SetCurrentHeadMesh (Variables|HairPawn|Head|SkeletalMesh|GetHeadMesh_Happiness))
      (goto _label))
    (:NewEnumerator4
      (Variables|HairPawn|Head|SkeletalMesh|SetCurrentHeadMesh (Variables|HairPawn|Head|SkeletalMesh|GetHeadMesh_Sadness))
      (goto _label))
    (:NewEnumerator5
      (Variables|HairPawn|Head|SkeletalMesh|SetCurrentHeadMesh (Variables|HairPawn|Head|SkeletalMesh|GetHeadMesh_Surprise))
      (goto _label))
    (:NewEnumerator7
      _))
  ;[0.147 0.008568 0.2195] Set StaticMesh visible
  (Rendering|SetVisibility (Variables|HairPawn|Head|SkeletalMesh|GetCurrentHeadMesh) true true))

(fn SwitchHeadMeshMaterial
  (bind _currentheadmesh (Variables|HairPawn|Head|SkeletalMesh|GetCurrentHeadMesh))
  (Utilities|FlowControl|Sequence
    (:then_0
      ;[0.147 0.008568 0.2195] Material of Face static mesh
      (bind _returnvalue (Rendering|Material|CreateDynamicMaterialInstance _currentheadmesh 0 (Rendering|Material|GetMaterial _currentheadmesh 0) "None" :!class /Script/Engine.PrimitiveComponent))
      (Variables|HairPawn|Head|Material|SetCurrentFaceMaterial _returnvalue))
    (:then_1
      ;[1 0.7704 0.1283] Material of Face Shader Lig (Temp)
      (switch Utilities|FlowControl|Switch|SwitchonE_FaceExpression (Variables|HairPawn|Head|GetCurrentExpression)
        (:NewEnumerator0
          (Variables|HairPawn|Head|Material|ShaderRig|SetCurrentFaceShaderRigMaterial (Variables|HairPawn|Head|Material|ShaderRig|GetShaderRig_Anger))
          ;[1 1 1] Mask Map
          (Variables|HairPawn|Head|Material|MaskMap|SetCurrentMaskMapMaterial (Variables|HairPawn|Head|Material|MaskMap|GetMaskMap_Anger)))
        (:NewEnumerator1
          (Variables|HairPawn|Head|Material|ShaderRig|SetCurrentFaceShaderRigMaterial (Variables|HairPawn|Head|Material|ShaderRig|GetShaderRig_Disgust))
          (Variables|HairPawn|Head|Material|MaskMap|SetCurrentMaskMapMaterial (Variables|HairPawn|Head|Material|MaskMap|GetMaskMap_Disgust)))
        (:NewEnumerator2
          (Variables|HairPawn|Head|Material|ShaderRig|SetCurrentFaceShaderRigMaterial (Variables|HairPawn|Head|Material|ShaderRig|GetShaderRig_Fear))
          (Variables|HairPawn|Head|Material|MaskMap|SetCurrentMaskMapMaterial (Variables|HairPawn|Head|Material|MaskMap|GetMaskMap_Fear)))
        (:NewEnumerator3
          (Variables|HairPawn|Head|Material|ShaderRig|SetCurrentFaceShaderRigMaterial (Variables|HairPawn|Head|Material|ShaderRig|GetShaderRig_Happy))
          (Variables|HairPawn|Head|Material|MaskMap|SetCurrentMaskMapMaterial (Variables|HairPawn|Head|Material|MaskMap|GetMaskMap_Happy)))
        (:NewEnumerator4
          (Variables|HairPawn|Head|Material|ShaderRig|SetCurrentFaceShaderRigMaterial (Variables|HairPawn|Head|Material|ShaderRig|GetShaderRig_Sad))
          (Variables|HairPawn|Head|Material|MaskMap|SetCurrentMaskMapMaterial (Variables|HairPawn|Head|Material|MaskMap|GetMaskMap_Sad)))
        (:NewEnumerator5
          (Variables|HairPawn|Head|Material|ShaderRig|SetCurrentFaceShaderRigMaterial (Variables|HairPawn|Head|Material|ShaderRig|GetShaderRig_Surprise))
          (Variables|HairPawn|Head|Material|MaskMap|SetCurrentMaskMapMaterial (Variables|HairPawn|Head|Material|MaskMap|GetMaskMap_Surprise)))
        (:NewEnumerator7
          (Variables|HairPawn|Head|Material|ShaderRig|SetCurrentFaceShaderRigMaterial (Variables|HairPawn|Head|Material|ShaderRig|GetShaderRig_VitalSign))
          (Variables|HairPawn|Head|Material|MaskMap|SetCurrentMaskMapMaterial (Variables|HairPawn|Head|Material|MaskMap|GetMaskMap_VitalSign)))))))

(fn GetFaceRgbaTintColor
  (bind _returnvalue (Rendering|Material|GetVectorParameterValue (Variables|HairPawn|Head|Material|GetCurrentFaceMaterial) (Variables|HairPawn|Head|Material|GetParamName_BaseColorTint) :!class /Script/Engine.MaterialInstanceDynamic))
  (return _returnvalue))

(fn SetFaceRgbaTintColor
  (params (R :type Float%20%28double-precision%29) (G :type Float%20%28double-precision%29) (B :type Float%20%28double-precision%29) (A :type Float%20%28double-precision%29))
  (Utilities|FlowControl|Sequence
    (:then_0
      ;[1 1 1] 현재 색상값을 가져옴
      (bind _returnvalue (Rendering|Material|GetVectorParameterValue (Variables|HairPawn|Head|Material|GetCurrentFaceMaterial) (Variables|HairPawn|Head|Material|GetParamName_BaseColorTint) :!class /Script/Engine.MaterialInstanceDynamic))
      (Utilities|FlowControl|Sequence
        (:then_0
          (LocalVariables|SetNewR (.R (Utilities|Struct|BreakLinearColor _returnvalue))))
        (:then_1
          (LocalVariables|SetNewG (.G (Utilities|Struct|BreakLinearColor _returnvalue))))
        (:then_2
          (LocalVariables|SetNewB (.B (Utilities|Struct|BreakLinearColor _returnvalue))))
        (:then_3
          (LocalVariables|SetNewA (.A (Utilities|Struct|BreakLinearColor _returnvalue))))))
    (:then_1
      ;[1 1 1] 양수값인 경우 새로운 색상으로 적용 (음수값인 경우 현재 색상을 유지 시키게된다.)
      (if (not (< R 0.0))
        (LocalVariables|SetNewR R)))
    (:then_2
      (if (not (< G 0.0))
        (LocalVariables|SetNewG G)))
    (:then_3
      (if (not (< B 0.0))
        (LocalVariables|SetNewB B)))
    (:then_4
      (if (not (< A 0.0))
        (LocalVariables|SetNewA A)))
    (:then_5
      ;[1 1 1] 최종 색상
      (Rendering|Material|SetVectorParameterValue (Variables|HairPawn|Head|Material|GetCurrentFaceMaterial) (Variables|HairPawn|Head|Material|GetParamName_BaseColorTint) (Utilities|Struct|MakeLinearColor (LocalVariables|GetNewR) (LocalVariables|GetNewG) (LocalVariables|GetNewB) (LocalVariables|GetNewA)) :!class /Script/Engine.MaterialInstanceDynamic))))

(fn CreateandAttachHeadMesh
  (params (New%20Skeletal%20Mesh%20Asset :type Skeletal%20Mesh%20Object%20Reference) (AnimSequence :type Animation%20Asset%20Object%20Reference))
  (bind _returnvalue (AddComponent|AddSkeletalMeshComponent true (Variables|컴포넌트|GetInitHeadModelTransform)))
  (Components|SkeletalMesh|SetSkeletalMeshAsset _returnvalue New%20Skeletal%20Mesh%20Asset)
  (Utilities|FlowControl|Sequence
    (:then_0
      (bind _returnvalue_2 (Game|AddComponentbyClass "/Script/HairStrandsCore.GroomComponent" true (Math|Transform|MakeTransform "-104.000000,0.000000,2.000000")))
      (Transformation|AttachComponentToComponent _returnvalue_2 _returnvalue "None" "KeepRelative" "KeepRelative" "KeepRelative" false)
      (Class|GroomComponent|SetGroomAsset _returnvalue_2 "/Game/MetaHumans/MH_KJH/MaleHair_fro/Hair/Hair_S_SideSweptFringe.Hair_S_SideSweptFringe"))
    (:then_1
      (Components|Animation|SetAnimationMode _returnvalue "AnimationSingleNode" true)
      (Components|Animation|SetAnimation _returnvalue AnimSequence))
    (:then_2
      (Rendering|SetVisibility _returnvalue false true)
      (Rendering|SetCastShadow _returnvalue true)
      (Class|PrimitiveComponent|SetCastContactShadow _returnvalue true)
      (Class|PrimitiveComponent|SetAffectDynamicIndirectLighting _returnvalue true)
      (Rendering|SetAffectDistanceFieldLighting _returnvalue true))
    (:then_3
      (return _returnvalue))))

(fn GetFaceMorphTarget
  (return (Class|SkeletalMeshComponent|GetMorphTarget (Variables|HairPawn|Head|SkeletalMesh|GetCurrentHeadMesh) (Utilities|String|StringToName (Utilities|String|EnumtoString (Variables|HairPawn|Head|GetCurrentExpression))))))

(fn PlayFaceAnimation
  (params (Play :type Boolean))
  (bind _currentheadmesh (Variables|HairPawn|Head|SkeletalMesh|GetCurrentHeadMesh))
  (if Play
    (Audio|Components|Audio|Play _currentheadmesh true)
    (else
      (Audio|Components|Audio|Stop _currentheadmesh)
      (Components|Animation|SetPosition _currentheadmesh 0.0 false))))

(fn SetFaceAnimationPlayRate
  (params (Rate :type Float%20%28double-precision%29))
  (Components|Timeline|SetPlayRate (Variables|HairPawn|Head|SkeletalMesh|GetCurrentHeadMesh) Rate))

(fn SetVitalSignValue
  (params (Lerp%20Alpha :type Float%20%28double-precision%29))
  ;[0.147 0.008568 0.2195] Material (Static Mesh) - 3D
  (Rendering|Material|SetScalarParameterValue (Variables|HairPawn|Head|Material|GetCurrentFaceMaterial) (Variables|HairPawn|Head|Material|GetParamName_VitalSign) Lerp%20Alpha :!class /Script/Engine.MaterialInstanceDynamic)
  ;[1 0.7704 0.1283] Vital Sign - 2D
  (Rendering|Material|SetScalarParameterValue (Variables|HairPawn|Head|Material|ShaderRig|GetCurrentFaceShaderRigMaterial) (Variables|HairPawn|Head|Material|GetParamName_VitalSign) Lerp%20Alpha :!class /Script/Engine.MaterialInstanceDynamic))

(fn GetHeadMeshMaterial
  (return (Variables|HairPawn|Head|Material|GetCurrentFaceMaterial)))

(fn GetFaceShadeRrigMaterial
  (return (Variables|HairPawn|Head|Material|ShaderRig|GetCurrentFaceShaderRigMaterial)))

(fn SetFaceShaderRigValue
  (params (Lerp%20Alpha :type Float%20%28double-precision%29))
  ;[0.147 0.008568 0.2195] Material (Static Mesh) - 3D
  (Rendering|Material|SetScalarParameterValue (Variables|HairPawn|Head|Material|GetCurrentFaceMaterial) (Variables|HairPawn|Head|Material|GetParamName_ShaderRigAlpha) Lerp%20Alpha :!class /Script/Engine.MaterialInstanceDynamic)
  ;[1 0.7704 0.1283] Shader Lig - 2D
  (Rendering|Material|SetScalarParameterValue (Variables|HairPawn|Head|Material|ShaderRig|GetCurrentFaceShaderRigMaterial) (Variables|HairPawn|Head|Material|GetParamName_ShaderRigAlpha) Lerp%20Alpha :!class /Script/Engine.MaterialInstanceDynamic))

(fn ResetStateCurrentHeadMesh
  (bind _currentheadmesh (Variables|HairPawn|Head|SkeletalMesh|GetCurrentHeadMesh))
  (Rendering|SetVisibility _currentheadmesh false true)
  (Audio|Components|Audio|Stop _currentheadmesh)
  (Components|Animation|SetPosition _currentheadmesh 0.0 false)
  (HairPawn|Head|Animation|SetFaceMorphTarget 0.0)
  (HairPawn|Head|Material|SetFaceShaderRigValue 0.0))

(fn GetMaskMapMaterial
  (return (Variables|HairPawn|Head|Material|MaskMap|GetCurrentMaskMapMaterial)))

(fn ApplyPPG
  (params (PPG :type Float%20%28double-precision%29) (Alpha :type Float%20%28double-precision%29))
  (bind _returnvalue (Math|Float|Truncate PPG))
  (bind _ppg_data (Variables|PPG|GetPPG%20Data))
  (bind (_outdata _returnvalue_2) (Class|PpgDataParser|GetData _ppg_data _returnvalue))
  (if _returnvalue_2
    (HairPawn|Head|Material|SetFaceRgbaTintColor (.PPG (Utilities|Struct|BreakPPG_Data _outdata)) 1.0 1.0 1.0) ; Apply
    (else
      (HairPawn|Head|Material|SetFaceRgbaTintColor 1.0 1.0 1.0 1.0) ; Default Color
    )))

(fn ApplyPPGLoopCounter
  (PPG|ApplyPPG (Math|Conversions|ToFloat(Integer) (Variables|PPG|GetPPG%20Row%20Counter)) 0.0)
  (bind _result (Math|Integer|IncrementInt (Variables|PPG|GetPPG%20Row%20Counter))
    (:%20%20
      (Variables|PPG|SetPPG%20Row%20Counter (Math|Integer|%(Integer) _result (Variables|PPG|GetPPG%20Max%20Length))))))

(fn SetHairViewandSwitchFaceModel
  (params (HairView :type EHairView%20Enum :default "ShaderRig"))
  (bind _output_get (Variables|Default|SetCurrentHairView HairView))
  (switch Utilities|FlowControl|Switch|SwitchonEHairView _output_get
    (:ShaderRig
      ;[1 1 1] Mode : Shader Rig
      (CallFunction|SetHeadMatchModelVisibility false false)
      (Rendering|SetVisibility (Variables|HairPawn|Head|SkeletalMesh|GetCurrentHeadMesh) true true))
    (:HairMatch
      ;[1 1 1] Mode : Head Match
      (CallFunction|SetAllShaderRigHeadMeshInvisible)
      (CallFunction|SetHeadMatchModelHair 0 (Variables|Default|GetSelected%20Hair%20Number)) ; Temp
    )))

(fn SetAllShaderRigHeadMeshInvisible
  (Utilities|FlowControl|Sequence
    (:then_0
      (Rendering|SetVisibility (Variables|HairPawn|Head|SkeletalMesh|GetHeadMesh_Anger) false true))
    (:then_1
      (Rendering|SetVisibility (Variables|HairPawn|Head|SkeletalMesh|GetHeadMesh_Disgust) false true))
    (:then_2
      (Rendering|SetVisibility (Variables|HairPawn|Head|SkeletalMesh|GetHeadMesh_Fear) false true))
    (:then_3
      (Rendering|SetVisibility (Variables|HairPawn|Head|SkeletalMesh|GetHeadMesh_Happiness) false true))
    (:then_4
      (Rendering|SetVisibility (Variables|HairPawn|Head|SkeletalMesh|GetHeadMesh_Sadness) false true))
    (:then_5
      (Rendering|SetVisibility (Variables|HairPawn|Head|SkeletalMesh|GetHeadMesh_Surprise) false true))))

(fn SetHeadMatchModelVisibility
  (params (Visibility :type Boolean) (Visible%20Man :type Boolean))
  (bind _returnvalue (not Visible%20Man))
  (if Visibility
    (Utilities|FlowControl|Sequence
      (:then_0
        ;[1 1 1] Man
        (Rendering|SetVisibility (Variables|Default|GetFace1) Visible%20Man false)
        (Rendering|SetVisibility (Variables|Default|GetEyelashes1) Visible%20Man false))
      (:then_1
        ;[1 1 1] Woman
        (Rendering|SetVisibility (Variables|MetaHuman|GetFace) _returnvalue false)
        (Rendering|SetVisibility (Variables|MetaHuman|GetEyelashes) _returnvalue false)))
    (else
      (Utilities|FlowControl|Sequence
        (:then_0
          ;[1 1 1] Man
          (Rendering|SetVisibility (Variables|Default|GetFace1) false false)
          (Rendering|SetVisibility (Variables|Default|GetEyelashes1) false false))
        (:then_1
          ;[1 1 1] Woman
          (Rendering|SetVisibility (Variables|MetaHuman|GetFace) false false)
          (Rendering|SetVisibility (Variables|MetaHuman|GetEyelashes) false false))
        (:then_2
          (CallFunction|SetAllHeadMatchHairInvisible))))))

(fn SetHeadMatchModelHair
  (params (Hair%20Asset :type Groom%20Asset%20Object%20Reference) (Item%20Index :type Integer))
  (CallFunction|SetAllHeadMatchHairInvisible)
  (bind _output_get (Variables|Default|SetSelected%20Hair%20Number Item%20Index))
  (switch int _output_get
    (:0
      ;[1 1 1] Woman
      (Rendering|SetVisibility (Variables|Default|Get01_womanhair_short) true true)
      (CallFunction|SetHeadMatchModelVisibility true false :!label _label))
    (:1
      (Rendering|SetVisibility (Variables|Default|Get02_woman_bob01) true true)
      (goto _label))
    (:2
      (Rendering|SetVisibility (Variables|Default|Get03_woman_bob02) true true)
      (goto _label))
    (:3
      (Rendering|SetVisibility (Variables|Default|Get04_woman_bob03) true true)
      (goto _label))
    (:4
      (Rendering|SetVisibility (Variables|Default|Get05_womanhair) true true)
      (goto _label))
    (:5
      (Rendering|SetVisibility (Variables|Default|Get06_womanhairmedium) true true)
      (goto _label))
    (:6
      (Rendering|SetVisibility (Variables|Default|Get07_womanhair_longstra) true true)
      (goto _label))
    (:7
      (Rendering|SetVisibility (Variables|Default|Get08_womanhair_longwave) true true)
      (goto _label))
    (:8
      (Rendering|SetVisibility (Variables|Default|Get09_womanhair_ponytail) true true)
      (goto _label))
    (:9
      (Rendering|SetVisibility (Variables|Default|Get10_womanhair_pigtail) true true)
      (goto _label))
    (:10
      (Rendering|SetVisibility (Variables|Default|Get11_womanhair_strong) true true)
      (goto _label))
    (:11
      (Rendering|SetVisibility (Variables|Default|Get12_womanhair_afro) true true)
      (goto _label))
    (:12
      ;[1 1 1] Man
      (Rendering|SetVisibility (Variables|Default|Get01_manhair_short) true true)
      (CallFunction|SetHeadMatchModelVisibility true true :!label _label_2))
    (:13
      (Rendering|SetVisibility (Variables|Default|Get02_manhair_short2) true true)
      (goto _label_2))
    (:14
      (Rendering|SetVisibility (Variables|Default|Get03_manhair_middle) true true)
      (goto _label_2))
    (:15
      (Rendering|SetVisibility (Variables|Default|Get04_manhair_long) true true)
      (goto _label_2))))

(fn SetHeadMatchHairInvisible
  (params (Is%20Man :type Boolean))
  (if Is%20Man
    ;[1 1 1] Man
    (Rendering|SetVisibility (Variables|Default|Get01_manhair_short) false false)
    (Rendering|SetVisibility (Variables|Default|Get02_manhair_short2) false false)
    (Rendering|SetVisibility (Variables|Default|Get03_manhair_middle) false false)
    (Rendering|SetVisibility (Variables|Default|Get04_manhair_long) false false)
    (else
      ;[1 1 1] Woman
      (Utilities|FlowControl|Sequence
        (:then_0
          (Rendering|SetVisibility (Variables|Default|Get01_womanhair_short) false false)
          (Rendering|SetVisibility (Variables|Default|Get02_woman_bob01) false false)
          (Rendering|SetVisibility (Variables|Default|Get03_woman_bob02) false false)
          (Rendering|SetVisibility (Variables|Default|Get04_woman_bob03) false false))
        (:then_1
          (Rendering|SetVisibility (Variables|Default|Get05_womanhair) false false)
          (Rendering|SetVisibility (Variables|Default|Get06_womanhairmedium) false false)
          (Rendering|SetVisibility (Variables|Default|Get07_womanhair_longstra) false false)
          (Rendering|SetVisibility (Variables|Default|Get08_womanhair_longwave) false false))
        (:then_2
          (Rendering|SetVisibility (Variables|Default|Get09_womanhair_ponytail) false false)
          (Rendering|SetVisibility (Variables|Default|Get10_womanhair_pigtail) false false)
          (Rendering|SetVisibility (Variables|Default|Get11_womanhair_strong) false false)
          (Rendering|SetVisibility (Variables|Default|Get12_womanhair_afro) false false))))))

(fn SetAllHeadMatchHairInvisible
  (Utilities|FlowControl|Sequence
    (:then_0
      ;[1 1 1] Man
      (Rendering|SetVisibility (Variables|Default|Get01_manhair_short) false false)
      (Rendering|SetVisibility (Variables|Default|Get02_manhair_short2) false false)
      (Rendering|SetVisibility (Variables|Default|Get03_manhair_middle) false false)
      (Rendering|SetVisibility (Variables|Default|Get04_manhair_long) false false))
    (:then_1
      ;[1 1 1] Woman
      (Rendering|SetVisibility (Variables|Default|Get01_womanhair_short) false false)
      (Rendering|SetVisibility (Variables|Default|Get02_woman_bob01) false false)
      (Rendering|SetVisibility (Variables|Default|Get03_woman_bob02) false false)
      (Rendering|SetVisibility (Variables|Default|Get04_woman_bob03) false false))
    (:then_2
      (Rendering|SetVisibility (Variables|Default|Get05_womanhair) false false)
      (Rendering|SetVisibility (Variables|Default|Get06_womanhairmedium) false false)
      (Rendering|SetVisibility (Variables|Default|Get07_womanhair_longstra) false false)
      (Rendering|SetVisibility (Variables|Default|Get08_womanhair_longwave) false false))
    (:then_3
      (Rendering|SetVisibility (Variables|Default|Get09_womanhair_ponytail) false false)
      (Rendering|SetVisibility (Variables|Default|Get10_womanhair_pigtail) false false)
      (Rendering|SetVisibility (Variables|Default|Get11_womanhair_strong) false false)
      (Rendering|SetVisibility (Variables|Default|Get12_womanhair_afro) false false))))